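; DarkForestAvatar is a flying player character with mouse-driven rotation and camera-relative movement.
; BeginPlay sets the movement mode to Flying, and holding the middle mouse button lets Turn and LookUp rotate the actor.
; Yaw and pitch are applied in opposite CombineRotators orders, separating world-space turning from local pitching.
; Each Space press adds one forced, heavily scaled movement input along camera vectors weighted by the MoveForward and MoveRight axes.
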(event EventTick
  (params (DeltaSeconds :type Float%20%28single-precision%29)))

(event EventBeginPlay
  (Pawn|Components|CharacterMovement|SetMovementMode (Variables|Character|GetCharacterMovement) "MOVE_Flying" 0))

(event Input|AxisEvents|InputAxisLookUp
  (params (AxisValue :type Float%20%28single-precision%29))
  (if (Variables|Default|GetCan%20Rotate)
    (Transformation|SetActorRotation (Math|Rotator|CombineRotators (Math|Rotator|MakeRotator 0.0 AxisValue 0.0) (Transformation|GetActorRotation)))))

(event Input|AxisEvents|InputAxisTurn
  (params (AxisValue :type Float%20%28single-precision%29))
  (if (Variables|Default|GetCan%20Rotate)
    (Transformation|SetActorRotation (Math|Rotator|CombineRotators (Transformation|GetActorRotation) (Math|Rotator|MakeRotator 0.0 0.0 AxisValue)))))

(event Input|KeyboardEvents|SpaceBar
  (params (Key :type Key%20Structure :default "None"))
  (bind _camera (Variables|Default|GetCamera))
  (:Pressed
    (Pawn|Input|AddMovementInput (+ (* (Math|Vector|GetForwardVector _camera) (Input|AxisValues|GetMoveForward)) (* (Math|Vector|GetRightVector _camera) (Input|AxisValues|GetMoveRight))) 1e+04 true)))

(event Input|MouseEvents|MiddleMouseButton
  (params (Key :type Key%20Structure :default "None"))
  (:Pressed
    (Variables|Default|SetCan%20Rotate true))
  (:Released
    (Variables|Default|SetCan%20Rotate false)))

(fn ConstructionScript)