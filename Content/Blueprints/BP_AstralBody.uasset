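; Player-controlled flying astral body that travels between stars on the star map and resumes at the star location saved in the GameInstance.
; Space launches it along camera-relative input with drift steering, or, near an overlapped BP_Star, lerps it onto that star's Roost, followed by a short relaunch cooldown.
; Holding CameraRotate orbits the spring arm.
; The wheel zooms, and zooming fully in while stopped at a star saves its location and opens Pocket.
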(event OnComponentBeginOverlap(Collision)
  (params (OverlappedComponent :type Primitive%20Component%20Object%20Reference) (OtherActor :type Actor%20Object%20Reference) (OtherComp :type Primitive%20Component%20Object%20Reference) (OtherBodyIndex :type Integer) (bFromSweep :type Boolean) (SweepResult :type Hit%20Result%20Structure%20%28by%20ref%29))
  (bind _asbp_star (Utilities|Casting|CastToBP_Star OtherActor))
  (Variables|Default|SetNearest%20Star _asbp_star))

(event OnComponentEndOverlap(Collision)
  (params (OverlappedComponent :type Primitive%20Component%20Object%20Reference) (OtherActor :type Actor%20Object%20Reference) (OtherComp :type Primitive%20Component%20Object%20Reference) (OtherBodyIndex :type Integer))
  (Variables|Default|SetNearest%20Star 0))

(event EventTick
  (params (DeltaSeconds :type Float%20%28single-precision%29))
  (bind _returnvalue (Transformation|GetActorLocation))
  (bind _target_vector (Variables|Default|GetTarget%20Vector))
  (if (Variables|Default|GetMoving)
    (Pawn|Input|AddMovementInput (Math|Vector|Lerp(Vector) (Variables|Default|GetMovement%20Vector) (+ (CallFunction|DriftVector) (Variables|Default|GetMovement%20Vector)) (* DeltaSeconds 3e+01)) (Variables|Default|GetMovement%20Speed) false)
    (elif (Variables|Default|GetSettling)
      (Transformation|SetActorLocation (Math|Vector|Lerp(Vector) _returnvalue _target_vector (* DeltaSeconds 5.0)) false false)
      (if (< (Math|Vector|Distance(Vector) _returnvalue _target_vector) 1e+02)
        (Variables|Default|SetSettling false)
        (Variables|Default|SetResettle%20Counter 0.5))
      (else
        (CallFunction|ResetResettle DeltaSeconds)))))

(event EventBeginPlay
  (Utilities|FlowControl|Sequence
    (:then_0
      (bind _asneanderthal_instance (Utilities|Casting|CastToNeanderthalInstance (Game|GetGameInstance)))
      (Variables|Default|SetGame%20Instance _asneanderthal_instance)
      (if (not (Math|Vector|Equal(Vector) (Variables|/Game/Blueprints/NeanderthalInstance.NeanderthalInstance_C|GetCurrent%20Star%20Location _asneanderthal_instance) "0, 0, 0" 0.0001))
        (Transformation|SetWorldLocation (Variables|Collision|GetCapsuleComponent) (Variables|/Game/Blueprints/NeanderthalInstance.NeanderthalInstance_C|GetCurrent%20Star%20Location _asneanderthal_instance) true true)))
    (:then_1
      (Pawn|Components|CharacterMovement|SetMovementMode (Variables|Character|GetCharacterMovement) "MOVE_Flying" 0)
      (bind _returnvalue (UserInterface|CreateWidget "/Game/UI/Canvas.Canvas_C"))
      (UserInterface|Viewport|AddtoViewport _returnvalue 0)
      (Variables|Default|SetCanvas _returnvalue))
    (:then_2
      (Input|SetInputModeGameOnly (Game|GetPlayerController 0)))))

(event Input|ActionEvents|InputActionCameraRotate
  (params (Key :type Key%20Structure :default "None"))
  (:Pressed
    (Variables|Default|SetCan%20Rotate true))
  (:Released
    (Variables|Default|SetCan%20Rotate false)))

(event Input|AxisEvents|InputAxisLookUp
  (params (AxisValue :type Float%20%28single-precision%29))
  (if (Variables|Default|GetCan%20Rotate)
    (Transformation|SetWorldRotation (Variables|Default|GetSpringArm) (Math|Rotator|CombineRotators (Math|Rotator|MakeRotator 0.0 AxisValue 0.0) (Transformation|GetWorldRotation (Variables|Default|GetSpringArm))) false false)))

(event Input|AxisEvents|InputAxisTurn
  (params (AxisValue :type Float%20%28single-precision%29))
  (if (Variables|Default|GetCan%20Rotate)
    (Transformation|SetWorldRotation (Variables|Default|GetSpringArm) (Math|Rotator|CombineRotators (Transformation|GetWorldRotation (Variables|Default|GetSpringArm)) (Math|Rotator|MakeRotator 0.0 0.0 AxisValue)) false false)))

(event Input|KeyboardEvents|SpaceBar
  (params (Key :type Key%20Structure :default "None"))
  (:Pressed
    (if (Variables|Default|GetMoving)
      (bind _nearest_star (Variables|Default|GetNearest%20Star)
        (:then
          (Variables|Default|SetMoving false)
          (Variables|Default|SetTarget%20Vector (Transformation|GetWorldLocation (Variables|/Game/Blueprints/BP_Star.BP_Star_C|GetRoost _nearest_star)))
          (Variables|Default|SetSettling true)
          (Variables|/Script/Engine.MovementComponent|SetVelocity (Variables|Character|GetCharacterMovement) "0, 0, 0"))
        (:else))
      (elif (<= (Variables|Default|GetResettle%20Counter) 0.0)
        (CallFunction|EstablishMovementVector)
        (Variables|Default|SetMoving true)
        (Variables|Default|SetNearest%20Star 0)
        (Variables|/Script/Engine.SpringArmComponent|SetbEnableCameraLag (Variables|Default|GetSpringArm) true)))))

(event Input|MouseEvents|MouseWheelUp
  (params (Key :type Key%20Structure :default "None"))
  (:Pressed
    (if (> (Variables|/Script/Engine.SpringArmComponent|GetTargetArmLength (Variables|Default|GetSpringArm)) 8e+02)
      (Variables|/Script/Engine.SpringArmComponent|SetTargetArmLength (Variables|Default|GetSpringArm) (+ (Variables|/Script/Engine.SpringArmComponent|GetTargetArmLength (Variables|Default|GetSpringArm)) (* (Variables|Default|GetZoom%20Scale) -1.0)))
      (elif (not (Variables|Default|GetMoving))
        (bind _nearest_star (Variables|Default|GetNearest%20Star)
          (:then
            (Utilities|FlowControl|Delay 0.75)
            (Variables|/Game/Blueprints/NeanderthalInstance.NeanderthalInstance_C|SetCurrent%20Star%20Location (Variables|Default|GetGame%20Instance) (Transformation|GetWorldLocation (Variables|/Game/Blueprints/BP_Star.BP_Star_C|GetRoost _nearest_star)))
            (Variables|/Script/Engine.SpringArmComponent|SetbEnableCameraLag (Variables|Default|GetSpringArm) false)
            (Game|OpenLevel(byName) "Pocket"))
          (:else))))))

(event Input|MouseEvents|MouseWheelDown
  (params (Key :type Key%20Structure :default "None"))
  (:Pressed
    (if (< (Variables|/Script/Engine.SpringArmComponent|GetTargetArmLength (Variables|Default|GetSpringArm)) 7e+03)
      (Variables|/Script/Engine.SpringArmComponent|SetTargetArmLength (Variables|Default|GetSpringArm) (+ (Variables|/Script/Engine.SpringArmComponent|GetTargetArmLength (Variables|Default|GetSpringArm)) (Variables|Default|GetZoom%20Scale))))))

(fn ConstructionScript)

(fn ResetResettle
  (params (Delta%20Time :type Float%20%28single-precision%29))
  (if (> (Variables|Default|GetResettle%20Counter) 0.0)
    (Variables|Default|SetResettle%20Counter (- (Variables|Default|GetResettle%20Counter) Delta%20Time))))

(fn EstablishMovementVector
  (bind _returnvalue (Input|AxisValues|GetMoveForward))
  (bind _returnvalue_2 (Input|AxisValues|GetMoveRight))
  (bind _camera (Variables|Default|GetCamera))
  (bind _returnvalue_3 (Math|Vector|GetForwardVector _camera))
  (bind _returnvalue_4 (Math|Vector|GetRightVector _camera))
  (bind _returnvalue_5 (* _returnvalue_3 _returnvalue))
  (bind _returnvalue_6 (* _returnvalue_4 _returnvalue_2))
  (bind _returnvalue_7 (+ _returnvalue_5 _returnvalue_6))
  (Variables|Default|SetMovement%20Vector (Math|Vector|Normalize (Math|Vector|MakeVector (.x _returnvalue_7) (.y _returnvalue_7) 0.0))))

(fn DriftVector
  (bind _returnvalue (Input|AxisValues|GetMoveForward))
  (bind _returnvalue_2 (Input|AxisValues|GetMoveRight))
  (bind _camera (Variables|Default|GetCamera))
  (bind _returnvalue_3 (Math|Vector|GetForwardVector _camera))
  (bind _returnvalue_4 (Math|Vector|GetRightVector _camera))
  (bind _returnvalue_5 (* _returnvalue_3 _returnvalue))
  (bind _returnvalue_6 (* _returnvalue_4 _returnvalue_2))
  (bind _returnvalue_7 (+ _returnvalue_5 _returnvalue_6))
  (return (Math|Vector|Normalize (Math|Vector|MakeVector (.x _returnvalue_7) (.y _returnvalue_7) 0.0))))