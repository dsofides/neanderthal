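; Player character for the Neanderthal, walking with camera-relative movement and creating the Canvas UI on begin play.
; Holding CameraRotate lets look input orbit the spring arm, while movement follows only the camera's yaw.
; The mouse wheel zooms the arm within limits; scrolling out at the far limit opens the DarkForest level after a short delay.
; Star overlap is only a cast stub, and two movement-vector helpers go uncalled here.
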(event OnComponentBeginOverlap(Collision)
  (params (OverlappedComponent :type Primitive%20Component%20Object%20Reference) (OtherActor :type Actor%20Object%20Reference) (OtherComp :type Primitive%20Component%20Object%20Reference) (OtherBodyIndex :type Integer) (bFromSweep :type Boolean) (SweepResult :type Hit%20Result%20Structure%20%28by%20ref%29))
  (Utilities|Casting|CastToBP_Star OtherActor))

(event OnComponentEndOverlap(Collision)
  (params (OverlappedComponent :type Primitive%20Component%20Object%20Reference) (OtherActor :type Actor%20Object%20Reference) (OtherComp :type Primitive%20Component%20Object%20Reference) (OtherBodyIndex :type Integer)))

(event EventBeginPlay
  (Pawn|Components|CharacterMovement|SetMovementMode (Variables|Character|GetCharacterMovement) "MOVE_Walking" 0)
  (bind _returnvalue (UserInterface|CreateWidget "/Game/UI/Canvas.Canvas_C"))
  (UserInterface|Viewport|AddtoViewport _returnvalue 0)
  (Variables|Default|SetCanvas _returnvalue)
  (bind _asneanderthal_instance (Utilities|Casting|CastToNeanderthalInstance (Game|GetGameInstance)))
  (Variables|Default|SetGame%20Instance _asneanderthal_instance)
  (Transformation|SetRelativeLocation (Variables|Default|GetSpringArm) "0, 0,130.000000" false false))

(event Input|ActionEvents|InputActionCameraRotate
  (params (Key :type Key%20Structure :default "None"))
  (:Pressed
    (Variables|Default|SetCan%20Rotate true))
  (:Released
    (Variables|Default|SetCan%20Rotate false)))

(event Input|AxisEvents|InputAxisLookUp
  (params (AxisValue :type Float%20%28single-precision%29))
  (if (Variables|Default|GetCan%20Rotate)
    (Transformation|SetWorldRotation (Variables|Default|GetSpringArm) (Math|Rotator|CombineRotators (Math|Rotator|MakeRotator 0.0 AxisValue 0.0) (Transformation|GetWorldRotation (Variables|Default|GetSpringArm))) false false)))

(event Input|AxisEvents|InputAxisTurn
  (params (AxisValue :type Float%20%28single-precision%29))
  (if (Variables|Default|GetCan%20Rotate)
    (Transformation|SetWorldRotation (Variables|Default|GetSpringArm) (Math|Rotator|CombineRotators (Transformation|GetWorldRotation (Variables|Default|GetSpringArm)) (Math|Rotator|MakeRotator 0.0 0.0 AxisValue)) false false)))

(event Input|AxisEvents|InputAxisMoveForward
  (params (AxisValue :type Float%20%28single-precision%29))
  (Pawn|Input|AddMovementInput (Math|Vector|GetForwardVector (Math|Rotator|MakeRotator 0.0 0.0 (.Yaw (Math|Rotator|BreakRotator (Transformation|GetWorldRotation (Variables|Default|GetCamera)))))) AxisValue false))

(event Input|AxisEvents|InputAxisMoveRight
  (params (AxisValue :type Float%20%28single-precision%29))
  (Pawn|Input|AddMovementInput (Math|Vector|GetRightVector (Math|Rotator|MakeRotator 0.0 0.0 (.Yaw (Math|Rotator|BreakRotator (Transformation|GetWorldRotation (Variables|Default|GetCamera)))))) AxisValue false))

(event Input|KeyboardEvents|SpaceBar
  (params (Key :type Key%20Structure :default "None")))

(event Input|MouseEvents|MouseWheelUp
  (params (Key :type Key%20Structure :default "None"))
  (:Pressed
    (if (> (Variables|/Script/Engine.SpringArmComponent|GetTargetArmLength (Variables|Default|GetSpringArm)) 1.2e+03)
      (Variables|/Script/Engine.SpringArmComponent|SetTargetArmLength (Variables|Default|GetSpringArm) (+ (Variables|/Script/Engine.SpringArmComponent|GetTargetArmLength (Variables|Default|GetSpringArm)) (* (Variables|Default|GetZoom%20Scale) -1.0))))))

(event Input|MouseEvents|MouseWheelDown
  (params (Key :type Key%20Structure :default "None"))
  (:Pressed
    (if (< (Variables|/Script/Engine.SpringArmComponent|GetTargetArmLength (Variables|Default|GetSpringArm)) 7e+03)
      (Variables|/Script/Engine.SpringArmComponent|SetTargetArmLength (Variables|Default|GetSpringArm) (+ (Variables|/Script/Engine.SpringArmComponent|GetTargetArmLength (Variables|Default|GetSpringArm)) (Variables|Default|GetZoom%20Scale)))
      (else
        (Utilities|FlowControl|Delay 1.0)
        (Game|OpenLevel(byName) "DarkForest")))))

(fn ConstructionScript)

(fn EstablishMovementVector
  (bind _returnvalue (Input|AxisValues|GetMoveForward))
  (bind _returnvalue_2 (Input|AxisValues|GetMoveRight))
  (bind _camera (Variables|Default|GetCamera))
  (bind _returnvalue_3 (Math|Vector|GetForwardVector _camera))
  (bind _returnvalue_4 (Math|Vector|GetRightVector _camera))
  (bind _returnvalue_5 (* _returnvalue_3 _returnvalue))
  (bind _returnvalue_6 (* _returnvalue_4 _returnvalue_2))
  (bind _returnvalue_7 (+ _returnvalue_5 _returnvalue_6))
  (Variables|Default|SetMovement%20Vector (Math|Vector|Normalize (Math|Vector|MakeVector (.x _returnvalue_7) (.y _returnvalue_7) 0.0))))

(fn DriftVector
  (bind _returnvalue (Input|AxisValues|GetMoveForward))
  (bind _returnvalue_2 (Input|AxisValues|GetMoveRight))
  (bind _camera (Variables|Default|GetCamera))
  (bind _returnvalue_3 (Math|Vector|GetForwardVector _camera))
  (bind _returnvalue_4 (Math|Vector|GetRightVector _camera))
  (bind _returnvalue_5 (* _returnvalue_3 _returnvalue))
  (bind _returnvalue_6 (* _returnvalue_4 _returnvalue_2))
  (bind _returnvalue_7 (+ _returnvalue_5 _returnvalue_6))
  (return (Math|Vector|Normalize (Math|Vector|MakeVector (.x _returnvalue_7) (.y _returnvalue_7) 0.0))))